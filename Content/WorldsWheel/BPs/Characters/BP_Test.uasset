(event `self.ReceiveBeginPlay`
  (`self.EnableInput` (`GameplayStatics.GetPlayerController` 0))
  (bind _asgs_game_instance (cast `/Game/WorldsWheel/GameLogic/GS_GameInstance` (`GameplayStatics.GetGameInstance`)))
  (set `self.GameInstance` _asgs_game_instance))

(event `Key|H`
  (params (Key :type "Key Structure"))
  ;[1 1 1] Hidden
  (:`Pressed`
    (`/Engine/EditorBlueprintResources/StandardMacros.FlipFlop`
      (:`A`
        (bind _outactors (`GameplayStatics.GetAllActorsOfClass` "/Game/WorldsWheel/BPs/Characters/BP_Source.BP_Source_C"))
        (for _array_element _outactors
          (`self.SetActorHiddenInGame` _array_element true)))
      (:`B`
        (bind _outactors_2 (`GameplayStatics.GetAllActorsOfClass` "/Game/WorldsWheel/BPs/Characters/BP_Source.BP_Source_C"))
        (for _array_element_2 _outactors_2
          (`self.SetActorHiddenInGame` _array_element_2 false))))))

(event `Key|I`
  (params (Key :type "Key Structure"))
  (bind _tags_0 (`self.Tags_0`))
  ;[1 1 1] tags
  (:`Pressed`
    (`KismetArrayLibrary.Array_Insert` _tags_0 (`KismetStringLibrary.Conv_StringToName` (`KismetStringLibrary.Conv_IntToString` (`/Game/WorldsWheel/GameLogic/GS_GameInstance.Lvl` (`self.GameInstance`)))))
    (set `self.Tags` _tags_0)
    (`KismetSystemLibrary.PrintString` (`KismetStringLibrary.Conv_NameToString` (`|GetArrayItem` _tags_0)))))

(event `Key|K`
  (params (Key :type "Key Structure"))
  ;[1 1 1] tags select
  (:`Pressed`
    (bind _outactors (`GameplayStatics.GetAllActorsWithTag` "0"))
    (for _array_element _outactors
      (`KismetSystemLibrary.PrintString` (`KismetSystemLibrary.GetDisplayName` _array_element)))))

(event `Key|O`
  (params (Key :type "Key Structure"))
  (:`Pressed`
    (bind _returnvalue (`GameplayStatics.GetActorOfClass` "/Game/WorldsWheel/BPs/Characters/BP_Source.BP_Source_C"))
    (bind _returnvalue_2 (`GameplayStatics.GetActorOfClass` "/Game/WorldsWheel/BPs/Characters/BP_Portal.BP_Portal_C"))
    (bind (_returnvalue_roll _returnvalue_pitch _returnvalue_yaw) (`KismetMathLibrary.BreakRotator` (`KismetMathLibrary.Conv_VectorToRotator` (`KismetMathLibrary.GetDirectionUnitVector` (`self.K2_GetActorLocation` _returnvalue) (`self.K2_GetActorLocation` _returnvalue_2)))))
    (`SceneComponent.K2_SetWorldRotation` (`/Game/WorldsWheel/BPs/Characters/BP_Portal.Cone` _returnvalue_2) (`KismetMathLibrary.MakeRotator` _returnvalue_roll 90.0 _returnvalue_yaw) false false)))

(fn `UserConstructionScript`)