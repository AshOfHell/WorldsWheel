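; BP_Retranslator is a relay actor that siphons score from the nearest node, up to a cap, and displays its total on a widget.
; On BeginPlay, FindClosest picks the nearest source, other retranslator or portal tagged with the current level number and orients its cone along that line.
; A looping one-second timer moves points from that target, using GameInstance's PortalCounter for portals, and stops when full or drained.
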(event `self.ReceiveBeginPlay`
  (`|ExecutionSequence`
    (:`then_0`
      ;[1 1 1] HUD
      (bind _aswbp_info (cast `/Game/WorldsWheel/BPs/Widgets/WBP_Info` (`WidgetComponent.GetUserWidgetObject` (`self.Widget`))))
      (bind _output_get (set `self.WBPInfo` _aswbp_info))
      (set `/Game/WorldsWheel/BPs/Widgets/WBP_Info.Score` (`self.Score`) _output_get))
    (:`then_1`
      ;[1 1 1] Game State ref
      (bind _asgs_game_instance (cast `/Game/WorldsWheel/GameLogic/GS_GameInstance` (`GameplayStatics.GetGameInstance`)))
      (set `self.GameInstance` _asgs_game_instance))
    (:`then_2`
      ;[1 1 1] Logic
      (`self.FindClosest`)
      (if (>= (`self.Score`) 100)
        (`KismetSystemLibrary.K2_ClearAndInvalidateTimerHandle` (`self.Timer`))
        (else
          (bind _returnvalue (`KismetSystemLibrary.K2_SetTimerDelegate` (delegate `OnDrainage`) 1.0 true))
          (set `self.Timer` _returnvalue))))))

(event `self.ReceiveTick`
  (params (DeltaSeconds :type "Float (single-precision)"))
  ;[1 1 1] HUD
  (`TextBlock.SetText` (`/Game/WorldsWheel/BPs/Widgets/WBP_Info.TextBlock_0` (`self.WBPInfo`)) (`KismetTextLibrary.Conv_IntToText` (`self.Score`))))

(event `OnDrainage`
  ;[1 1 1] Logic
  (`self.RetranslatorDrainage` (`self.Closest Actor`)))

(fn `FindClosest`
  (locals (ClosestDistance :type "Float (double-precision)" :default 100000000.0) (ClosestActor :type "Actor Object Reference"))
  (bind (_returnvalue_roll _returnvalue_pitch _returnvalue_yaw) (`KismetMathLibrary.BreakRotator` (`KismetMathLibrary.Conv_VectorToRotator` (`KismetMathLibrary.GetDirectionUnitVector` (`self.K2_GetActorLocation` (`local.ClosestActor`)) (`self.K2_GetActorLocation` self)))))
  (`|ExecutionSequence`
    (:`then_0`
      (bind _outactors (`GameplayStatics.GetAllActorsOfClass` "/Game/WorldsWheel/BPs/Characters/BP_Source.BP_Source_C"))
      (for _array_element _outactors
        (if (`self.ActorHasTag` _array_element (`KismetStringLibrary.Conv_StringToName` (`KismetStringLibrary.Conv_IntToString` (`/Game/WorldsWheel/GameLogic/GS_GameInstance.Lvl` (`self.GameInstance`)))))
          (bind _returnvalue (`KismetMathLibrary.Vector_Distance` (`self.K2_GetActorLocation` _array_element) (`self.K2_GetActorLocation` self)))
          (if (< _returnvalue (`local.ClosestDistance`))
            (set `local.ClosestDistance` _returnvalue)
            (set `local.ClosestActor` _array_element)))))
    (:`then_1`
      (bind _outactors_2 (`GameplayStatics.GetAllActorsOfClass` "BP_Retranslator_C"))
      (for _array_element_2 _outactors_2
        (if (== _array_element_2 self)
          _
          (elif (`self.ActorHasTag` _array_element_2 (`KismetStringLibrary.Conv_StringToName` (`KismetStringLibrary.Conv_IntToString` (`/Game/WorldsWheel/GameLogic/GS_GameInstance.Lvl` (`self.GameInstance`)))))
            (bind _returnvalue_2 (`KismetMathLibrary.Vector_Distance` (`self.K2_GetActorLocation` _array_element_2) (`self.K2_GetActorLocation` self)))
            (if (< _returnvalue_2 (`local.ClosestDistance`))
              (set `local.ClosestDistance` _returnvalue_2)
              (set `local.ClosestActor` _array_element_2))))))
    (:`then_2`
      (bind _outactors_3 (`GameplayStatics.GetAllActorsOfClass` "/Game/WorldsWheel/BPs/Characters/BP_Portal.BP_Portal_C"))
      (for _array_element_3 _outactors_3
        (if (`self.ActorHasTag` _array_element_3 (`KismetStringLibrary.Conv_StringToName` (`KismetStringLibrary.Conv_IntToString` (`/Game/WorldsWheel/GameLogic/GS_GameInstance.Lvl` (`self.GameInstance`)))))
          (bind _returnvalue_3 (`KismetMathLibrary.Vector_Distance` (`self.K2_GetActorLocation` _array_element_3) (`self.K2_GetActorLocation` self)))
          (if (< _returnvalue_3 (`local.ClosestDistance`))
            (set `local.ClosestDistance` _returnvalue_3)
            (set `local.ClosestActor` _array_element_3)))))
    (:`then_3`
      (set `local.ClosestDistance` 1000000000.0))
    (:`then_4`
      (`/Engine/EditorBlueprintResources/StandardMacros.IsValid` (`local.ClosestActor`)
        (:`Is Valid`
          (`SceneComponent.K2_SetWorldRotation` (`self.Cone`) (`KismetMathLibrary.MakeRotator` _returnvalue_roll 90.0 _returnvalue_yaw) false false))))
    (:`then_5`
      (set `self.Closest Actor` (`local.ClosestActor`)))))

(fn `UserConstructionScript`)