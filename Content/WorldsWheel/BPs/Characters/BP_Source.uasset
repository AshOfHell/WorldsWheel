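; BP_Source is a Blueprint that displays its Score as text through a WBP_Info widget hosted in its Widget component.
; On BeginPlay it casts and caches the component's user widget, then copies Score into it.
; Every Tick it writes the current Score directly into the widget's TextBlock0, so the label is refreshed by polling rather than on change.
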(event `self.ReceiveBeginPlay`
  ;[1 1 1] Label
  (bind _aswbp_info (cast `/Game/WorldsWheel/BPs/Widgets/WBP_Info` (`WidgetComponent.GetUserWidgetObject` (`self.Widget`))))
  (bind _output_get (set `self.WBPInfo` _aswbp_info))
  (set `/Game/WorldsWheel/BPs/Widgets/WBP_Info.Score` (`self.Score`) _output_get))

(event `self.ReceiveTick`
  (params (DeltaSeconds :type "Float (single-precision)"))
  ;[1 1 1] Label
  (`TextBlock.SetText` (`/Game/WorldsWheel/BPs/Widgets/WBP_Info.TextBlock_0` (`self.WBPInfo`)) (`KismetTextLibrary.Conv_IntToText` (`self.Score`))))

(fn `UserConstructionScript`)