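; Player character that moves, looks and places Source, Retranslator and Portal actors across numbered virtual levels.
; Input actions spawn each actor ahead of the camera at a fixed height and tag it with the GameInstance's current level number.
; Next and previous level inputs change that number, stopping at zero, and reset the player's position.
; Levels are simulated by hiding all three actor types, then unhiding those tagged with the new number, without loading maps.
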(event `self.ReceiveBeginPlay`
  (bind _asgs_game_instance (cast `/Game/WorldsWheel/GameLogic/GS_GameInstance` (`GameplayStatics.GetGameInstance`)))
  (set `self.GameInstance` _asgs_game_instance))

(event `InputAxis|MoveForwardBackward`
  (params (AxisValue :type "Float (single-precision)"))
  ;[1 1 1] Movement
  (`self.AddMovementInput` (`self.GetActorForwardVector`) AxisValue))

(event `self.ReceiveTick`
  (params (DeltaSeconds :type "Float (single-precision)"))
  ;[1 1 1] Look
  (`self.AddControllerYawInput` (`self.GetInputAxisKeyValue`))
  (`self.AddControllerPitchInput` (* -1 (`self.GetInputAxisKeyValue`))))

(event `InputAxis|MoveLeftRight`
  (params (AxisValue :type "Float (single-precision)"))
  ;[1 1 1] Movement
  (`self.AddMovementInput` (`self.GetActorRightVector`) AxisValue))

(event `InputAction|SpawnSource`
  (params (Key :type "Key Structure"))
  (bind (_returnvalue_x _returnvalue_y) (`KismetMathLibrary.BreakVector` (+ (* (`KismetMathLibrary.Normal` (`SceneComponent.GetForwardVector` (`self.Camera`))) (100.0 100.0 0.0)) (`self.K2_GetActorLocation`))))
  ;[1 1 1] Spawn
  (:`Pressed`
    (bind _returnvalue (`|SpawnActorFromClass` "/Game/WorldsWheel/BPs/Characters/BP_Source.BP_Source_C" (`KismetMathLibrary.MakeTransform` (`KismetMathLibrary.MakeVector` _returnvalue_x _returnvalue_y 151.0)) "Undefined" "OverrideRootScale" null null))
    (`self.ActorTagging` _returnvalue)))

(event `InputAction|NextLvl`
  (params (Key :type "Key Structure"))
  ;[1 1 1] Lvl mngr
  (:`Pressed`
    (`self.NextLevel`)))

(event `InputAction|SpawnRetranslator`
  (params (Key :type "Key Structure"))
  (bind (_returnvalue_x _returnvalue_y) (`KismetMathLibrary.BreakVector` (+ (* (`KismetMathLibrary.Normal` (`SceneComponent.GetForwardVector` (`self.Camera`))) (100.0 100.0 0.0)) (`self.K2_GetActorLocation`))))
  ;[1 1 1] Spawn
  (:`Pressed`
    (bind _returnvalue (`|SpawnActorFromClass` "/Game/WorldsWheel/BPs/Characters/BP_Retranslator.BP_Retranslator_C" (`KismetMathLibrary.MakeTransform` (`KismetMathLibrary.MakeVector` _returnvalue_x _returnvalue_y 151.0)) "Undefined" "OverrideRootScale" null null))
    (`self.ActorTagging` _returnvalue)))

(event `InputAction|PrevLvl`
  (params (Key :type "Key Structure"))
  ;[1 1 1] Lvl mngr
  (:`Pressed`
    (`self.PrevLevel`)))

(event `InputAction|SpawnPortal`
  (params (Key :type "Key Structure"))
  (bind (_returnvalue_x _returnvalue_y) (`KismetMathLibrary.BreakVector` (+ (* (`KismetMathLibrary.Normal` (`SceneComponent.GetForwardVector` (`self.Camera`))) (100.0 100.0 0.0)) (`self.K2_GetActorLocation`))))
  ;[1 1 1] Spawn
  (:`Pressed`
    (bind _returnvalue (`|SpawnActorFromClass` "/Game/WorldsWheel/BPs/Characters/BP_Portal.BP_Portal_C" (`KismetMathLibrary.MakeTransform` (`KismetMathLibrary.MakeVector` _returnvalue_x _returnvalue_y 151.0)) "Undefined" "OverrideRootScale" null null))
    (`self.ActorTagging` _returnvalue)))

(fn `ActorTagging`
  (params (Actor :type "Actor Object Reference"))
  (bind _tagssource (`self.TagsSource`))
  (`KismetArrayLibrary.Array_Insert` _tagssource (`KismetStringLibrary.Conv_StringToName` (`KismetStringLibrary.Conv_IntToString` (`/Game/WorldsWheel/GameLogic/GS_GameInstance.Lvl` (`self.GameInstance`)))))
  (set `Actor.Tags` _tagssource Actor)
  (`KismetArrayLibrary.Array_Clear` _tagssource))

(fn `ChangeLvlActors`
  (`|ExecutionSequence`
    (:`then_0`
      (bind _outactors (`GameplayStatics.GetAllActorsOfClass` "/Game/WorldsWheel/BPs/Characters/BP_Source.BP_Source_C"))
      (for _array_element _outactors
        (`self.SetActorHiddenInGame` _array_element true)))
    (:`then_1`
      (bind _outactors_2 (`GameplayStatics.GetAllActorsOfClass` "/Game/WorldsWheel/BPs/Characters/BP_Retranslator.BP_Retranslator_C"))
      (for _array_element_2 _outactors_2
        (`self.SetActorHiddenInGame` _array_element_2 true)))
    (:`then_2`
      (bind _outactors_3 (`GameplayStatics.GetAllActorsOfClass` "/Game/WorldsWheel/BPs/Characters/BP_Portal.BP_Portal_C"))
      (for _array_element_3 _outactors_3
        (`self.SetActorHiddenInGame` _array_element_3 true)))
    (:`then_3`
      (bind _outactors_4 (`GameplayStatics.GetAllActorsWithTag` (`KismetStringLibrary.Conv_StringToName` (`KismetStringLibrary.Conv_IntToString` (`/Game/WorldsWheel/GameLogic/GS_GameInstance.Lvl` (`self.GameInstance`))))))
      (for _array_element_4 _outactors_4
        (`self.SetActorHiddenInGame` _array_element_4 false)))))

(fn `UserConstructionScript`)